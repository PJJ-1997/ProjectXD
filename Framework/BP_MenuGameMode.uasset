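; Lobby game mode for the multiplayer menu, tracking connected players' profiles, ready states, team IDs and the selected gamemode (Endless Wave, Free for All, Team Death Match).
; UpdateLobby pushes that state to each BP_MenuController and copies profiles into player states.
; Lobby characters spawn at free player spots, with meshes and skins from a customisation DataTable.
; Helpers enforce team sizes, deal players into teams by level and apply team-colour character overrides.
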(event Custom|UpdateLobby
  (params (PlayerNames :type Boolean) (UpdateSelection :type Boolean) (CharacterSelection :type Boolean) (PlayersReady :type Boolean) (Gamemode :type Boolean) (TeamIDs :type Boolean))
  (Utilities|Array|Clear (Variables|Default|GetAll_PlayerProfiles))
  (for (_array_element _array_index) (Variables|Default|GetAll_ConnectedPlayers)
    (Utilities|Array|SetArrayElem (Variables|Default|GetAll_PlayerProfiles) _array_index (Variables|/Game/Framework/BP_MenuController.BP_MenuController_C|GetPlayerProfileInfo _array_element) true)
    (bind _asbp_shooter_playerstate (Utilities|Casting|CastToBP_ShooterPlayerstate (Variables|/Script/Engine.Controller|GetPlayerState _array_element)))
    (Variables|/Game/Framework/BP_ShooterPlayerstate.BP_ShooterPlayerstate_C|SetS_PlayerProfile _asbp_shooter_playerstate (Variables|/Game/Framework/BP_MenuController.BP_MenuController_C|GetPlayerProfileInfo _array_element)))
  (for (_array_element_2 _array_index_2) (Variables|Default|GetAll_ConnectedPlayers)
    (if PlayerNames
      (Default|UpdatePlayerNames _array_element_2 (Variables|Default|GetAll_PlayerProfiles)))
    (if TeamIDs
      (Default|UpdateTeamIDs _array_element_2 (Variables|Default|GetAll_TeamIDs) Gamemode (Variables|Default|GetAutoAssignTeams)))
    (if UpdateSelection
      (Default|UpdateLevelSelection _array_element_2 (Variables|Default|GetSelectedLevelName)))
    (if CharacterSelection
      (CallFunction|UpdateSelectedCharacter _array_index_2))
    (if PlayersReady
      (Default|UpdatePlayerReady _array_element_2 (Variables|Default|GetIsPlayerReady)))
    (if Gamemode
      (Default|UpdateGamemode _array_element_2 (Variables|Default|GetSelectedGamemode) (Variables|Default|GetMaxTeamSize) (Variables|Default|GetNrOfTeams) (Variables|Default|GetAutoAssignTeams)))))

(event Custom|UpdateSelectedCharacter
  (params (PlayerIndex :type Integer))
  (bind _all_connectedplayers (Variables|Default|GetAll_ConnectedPlayers))
  (bind _all_connectedplayers_2 (Variables|Default|GetAll_ConnectedPlayers))
  (bind _all_playerprofiles (Variables|Default|GetAll_PlayerProfiles))
  (bind _output (Utilities|Array|Get(acopy) _all_connectedplayers PlayerIndex))
  (bind _output_2 (Utilities|Array|Get(acopy) _all_connectedplayers_2 PlayerIndex))
  (bind _output_3 (Utilities|Array|Get(acopy) _all_playerprofiles PlayerIndex))
  (if (== (Variables|/Game/Framework/BP_MenuController.BP_MenuController_C|GetLobbyCharacter_BP _output) 0)
    (bind _availableplayerspot (CallFunction|GetLobbyPlayerSpot))
    (Variables|/Game/Gameplay/Lobby_PlayerSpot_BP.Lobby_PlayerSpot_BP_C|SetIsSpotUsed _availableplayerspot true)
    ;[1 1 1] Owenr 노드에 따라서 다른 캐릭터를 선택할시 Mesh가 변경된다.(#20-> 40:54)
    (bind _returnvalue (Game|SpawnActorfromClass "/Game/Gameplay/lobby_Character_BP.lobby_Character_BP_C" (Transformation|GetActorTransform _availableplayerspot) "Undefined" "MultiplyWithRoot" _output 0))
    (Variables|/Game/Framework/BP_MenuController.BP_MenuController_C|SetLobbyCharacter_BP _output_2 _returnvalue)
    (Variables|/Game/Framework/BP_MenuController.BP_MenuController_C|SetLobbyPlayerSpot_BP _output_2 _availableplayerspot))
  (Default|MCSetPlayerName (Variables|/Game/Framework/BP_MenuController.BP_MenuController_C|GetLobbyCharacter_BP (Utilities|Array|Get(acopy) (Variables|Default|GetAll_ConnectedPlayers) PlayerIndex)) (.playername _output_3))
  (CallFunction|SetLobbyCharacterModelandSkin (Variables|/Game/Framework/BP_MenuController.BP_MenuController_C|GetLobbyCharacter_BP (Utilities|Array|Get(acopy) (Variables|Default|GetAll_ConnectedPlayers) PlayerIndex)) (.characterrowname _output_3) (.modelname _output_3) (.skinname _output_3)))

(event Custom|UpdateCharForController
  (params (Controller :type BP%20Menu%20Controller%20Object%20Reference) (PlayerProfile :type S%20Player%20Profile%20Structure))
  (bind _all_connectedplayers (Variables|Default|GetAll_ConnectedPlayers))
  (bind _returnvalue (Utilities|Array|FindItem _all_connectedplayers Controller))
  (Utilities|Array|SetArrayElem (Variables|Default|GetAll_PlayerProfiles) _returnvalue PlayerProfile true)
  (bind _asbp_shooter_playerstate (Utilities|Casting|CastToBP_ShooterPlayerstate (Variables|/Script/Engine.Controller|GetPlayerState Controller)))
  (Variables|/Game/Framework/BP_ShooterPlayerstate.BP_ShooterPlayerstate_C|SetS_PlayerProfile _asbp_shooter_playerstate PlayerProfile)
  (CallFunction|UpdateSelectedCharacter _returnvalue))

(event Custom|PreviewCharacterForController
  (params (Controller :type BP%20Menu%20Controller%20Object%20Reference) (CharRowName :type Name) (ModelName :type Name) (SkinName :type Name))
  (bind _lobbycharacter_bp (Variables|/Game/Framework/BP_MenuController.BP_MenuController_C|GetLobbyCharacter_BP Controller))
  (bind _returnvalue (Utilities|GetDataTableRow "/Game/Player/CharCustomisationm_Table.CharCustomisationm_Table" CharRowName)
    (:then
      (Default|ClientSetCharacterMesh _lobbycharacter_bp (.Model (Utilities|Struct|BreakS_ModelAndSkins (.Value (Utilities|Map|Find (.ModelsAndSkins (Utilities|Struct|BreakS_CharCustomisation _returnvalue)) ModelName)))))
      (Default|ClientPlayMeshAnim _lobbycharacter_bp (.LobbyAnimation (Utilities|Struct|BreakS_ModelAndSkins (.Value (Utilities|Map|Find (.ModelsAndSkins (Utilities|Struct|BreakS_CharCustomisation _returnvalue)) ModelName)))))
      (if (.Use_Skin0 (Utilities|Struct|BreakS_ModelAndSkins (.Value (Utilities|Map|Find (.ModelsAndSkins (Utilities|Struct|BreakS_CharCustomisation _returnvalue)) ModelName))))
        (Default|ClientSetSkinMaterial _lobbycharacter_bp (.Skin0_MaterialSlot (Utilities|Struct|BreakS_ModelAndSkins (.Value (Utilities|Map|Find (.ModelsAndSkins (Utilities|Struct|BreakS_CharCustomisation _returnvalue)) ModelName)))) (.Value (Utilities|Map|Find (.Skin0_Skins (Utilities|Struct|BreakS_ModelAndSkins (.Value (Utilities|Map|Find (.ModelsAndSkins (Utilities|Struct|BreakS_CharCustomisation _returnvalue)) ModelName)))) SkinName))))
      (if (.Use_Skin1 (Utilities|Struct|BreakS_ModelAndSkins (.Value (Utilities|Map|Find (.ModelsAndSkins (Utilities|Struct|BreakS_CharCustomisation _returnvalue)) ModelName))))
        (Default|ClientSetSkinMaterial _lobbycharacter_bp (.Skin1_MaterialSlot (Utilities|Struct|BreakS_ModelAndSkins (.Value (Utilities|Map|Find (.ModelsAndSkins (Utilities|Struct|BreakS_CharCustomisation _returnvalue)) ModelName)))) (.Value (Utilities|Map|Find (.Skin1_Skins (Utilities|Struct|BreakS_ModelAndSkins (.Value (Utilities|Map|Find (.ModelsAndSkins (Utilities|Struct|BreakS_CharCustomisation _returnvalue)) ModelName)))) SkinName)))))))

(event Custom|SetPlayerReady
  (params (PlayerController :type BP%20Menu%20Controller%20Object%20Reference) (IsReady :type Boolean))
  (Utilities|Array|SetArrayElem (Variables|Default|GetIsPlayerReady) (Utilities|Array|FindItem (Variables|Default|GetAll_ConnectedPlayers) PlayerController) IsReady)
  (CallFunction|UpdateLobby false false false true false false))

(event Custom|SetSelectedGamemode
  (params (SelectedGamemode :type E_GameModes%20Enum :default "NewEnumerator0") (MaxTeamSiez :type Integer) (NrOfTeams :type Integer) (AutoAssignTemas :type Boolean))
  (bind _all_teamids (Variables|Default|GetAll_TeamIDs))
  (bind _output_get (Variables|Default|SetSelectedGamemode SelectedGamemode))
  (if (and (== AutoAssignTemas true) (== (Variables|Default|GetAutoAssignTeams) false))
    (for (_ _array_index) _all_teamids
      (Utilities|Array|SetArrayElem _all_teamids _array_index 0)))
  (Variables|Default|SetAutoAssignTeams AutoAssignTemas)
  (switch Utilities|FlowControl|Switch|SwitchonE_GameModes _output_get
    (:NewEnumerator0
      (Variables|Default|SetNrOfTeams NrOfTeams)
      (Variables|Default|SetMaxTeamSize MaxTeamSiez))
    (:NewEnumerator1
      (if (< MaxTeamSiez (Utilities|Array|Length (Variables|Default|GetAll_ConnectedPlayers)))
        _
        (else
          (Variables|Default|SetNrOfTeams NrOfTeams)
          (Variables|Default|SetMaxTeamSize MaxTeamSiez))))
    (:NewEnumerator2
      (if (< (* MaxTeamSiez NrOfTeams) (Utilities|Array|Length (Variables|Default|GetAll_ConnectedPlayers)))
        _
        (else
          (Variables|Default|SetNrOfTeams NrOfTeams)
          (Variables|Default|SetMaxTeamSize MaxTeamSiez)
          (bind _idsoverwrite (CallFunction|CheckTeamIDs))))))
  (CallFunction|UpdateLobby false false false false true _idsoverwrite))

(event Custom|SetPlayerTeamID
  (params (PlayerController :type BP%20Menu%20Controller%20Object%20Reference) (PreferedTeamID :type Integer))
  (bind _canjoin (CallFunction|CanJoinTeam PreferedTeamID))
  (if _canjoin
    (Utilities|Array|SetArrayElem (Variables|Default|GetAll_TeamIDs) (Utilities|Array|FindItem (Variables|Default|GetAll_ConnectedPlayers) PlayerController) PreferedTeamID)
    (CallFunction|UpdateLobby false false false false false true)))

(event EventHandleStartingNewPlayer
  (params (NewPlayer :type Player%20Controller%20Object%20Reference))
  (bind _returnvalue (Game|GetCurrentLevelName true))
  (switch string _returnvalue
    (:LobbyMenu_Map
      (bind _asbp_menu_controller (Utilities|Casting|CastToBP_MenuController NewPlayer))
      (bind _returnvalue_2 (Utilities|Array|Add (Variables|Default|GetAll_ConnectedPlayers) _asbp_menu_controller))
      (Utilities|Array|SetArrayElem (Variables|Default|GetIsPlayerReady) _returnvalue_2 false true)
      (Utilities|Array|SetArrayElem (Variables|Default|GetAll_TeamIDs) _returnvalue_2 0 true)
      (Default|CreateLobbyMenu _asbp_menu_controller)
      (Default|InitialSetup _asbp_menu_controller))))

(event EventOnLogout
  (params (ExitingController :type Controller%20Object%20Reference))
  (bind _asbp_menu_controller (Utilities|Casting|CastToBP_MenuController ExitingController))
  (if (== (Variables|/Game/Framework/BP_MenuController.BP_MenuController_C|GetLobbyCharacter_BP _asbp_menu_controller) 0)
    _
    (else
      (Actor|DestroyActor (Variables|/Game/Framework/BP_MenuController.BP_MenuController_C|GetLobbyCharacter_BP _asbp_menu_controller))
      (Variables|/Game/Gameplay/Lobby_PlayerSpot_BP.Lobby_PlayerSpot_BP_C|SetIsSpotUsed (Variables|/Game/Framework/BP_MenuController.BP_MenuController_C|GetLobbyPlayerSpot_BP _asbp_menu_controller) false)))
  (Utilities|Array|RemoveIndex (Variables|Default|GetIsPlayerReady) (Utilities|Array|FindItem (Variables|Default|GetAll_ConnectedPlayers) _asbp_menu_controller))
  (Utilities|Array|RemoveIndex (Variables|Default|GetAll_TeamIDs) (Utilities|Array|FindItem (Variables|Default|GetAll_ConnectedPlayers) _asbp_menu_controller))
  (Utilities|Array|RemoveIndex (Variables|Default|GetAll_ConnectedPlayers) (Utilities|Array|FindItem (Variables|Default|GetAll_ConnectedPlayers) _asbp_menu_controller))
  (CallFunction|UpdateLobby true false true true true true))

(fn ConstructionScript)

(fn GetLobbyPlayerSpot
  (if (== (Utilities|Array|Length (Variables|Default|GetALL_Lobby_PlayerSpots)) 0)
    (bind _outactors (Actor|GetAllActorsOfClass "/Game/Gameplay/Lobby_PlayerSpot_BP.Lobby_PlayerSpot_BP_C"))
    (Variables|Default|SetALL_Lobby_PlayerSpots _outactors))
  (bind _array_element (Utilities|Array|ForEachLoopwithBreak (Variables|Default|GetALL_Lobby_PlayerSpots) :!label _label)
    (:LoopBody
      (if (not (Variables|/Game/Gameplay/Lobby_PlayerSpot_BP.Lobby_PlayerSpot_BP_C|GetIsSpotUsed _array_element))
        (goto _label Break)))
    (:Completed
      (return _array_element))))

(fn SendChatMessage
  (params (Message :type Text))
  (for _array_element (Variables|Default|GetAll_ConnectedPlayers)
    (Default|UpdateChatBox _array_element Message)))

(fn CanJoinTeam
  (params (TeamID :type Integer))
  (for _array_element (Variables|Default|GetAll_TeamIDs)
    (if (== _array_element TeamID)
      (Math|Integer|IncrementInt (LocalVariables|GetLcl_PlayerCount))))
  (if (< (LocalVariables|GetLcl_PlayerCount) (Variables|Default|GetMaxTeamSize))
    (return true)
    (else
      (return false))))

(fn CheckTeamIDs
  (for (_array_element _array_index) (Variables|Default|GetAll_TeamIDs)
    (if (>= _array_element (Variables|Default|GetNrOfTeams))
      (LocalVariables|SetLcl_TeamToCheck 0)
      (LocalVariables|SetLcl_playersInThisTeam 0 :!label _label)
      (for _array_element_2 (Variables|Default|GetAll_TeamIDs)
        (if (== _array_element_2 (LocalVariables|GetLcl_TeamToCheck))
          (Math|Integer|IncrementInt (LocalVariables|GetLcl_playersInThisTeam))))
      (if (< (LocalVariables|GetLcl_playersInThisTeam) (Variables|Default|GetMaxTeamSize))
        (Utilities|Array|SetArrayElem (Variables|Default|GetAll_TeamIDs) _array_index (LocalVariables|GetLcl_TeamToCheck) true)
        (LocalVariables|SetLcl_IDsOverWrite true)
        (else
          (Math|Integer|IncrementInt (LocalVariables|GetLcl_TeamToCheck)
            (:%20%20
              (if (not (== (LocalVariables|GetLcl_TeamToCheck) (Variables|Default|GetNrOfTeams)))
                (goto _label))))))))
  (for _array_element_3 (Variables|Default|GetAll_TeamIDs)
    (Utilities|Array|SetArrayElem (LocalVariables|GetLcl_TeamCounts) _array_element_3 (+ (Utilities|Array|Get(acopy) (LocalVariables|GetLcl_TeamCounts) _array_element_3) 1) true))
  (for (_array_element_4 _array_index_2) (LocalVariables|GetLcl_TeamCounts)
    (if (> _array_element_4 (Variables|Default|GetMaxTeamSize)) :!label _label_2
      (LocalVariables|SetLcl_TeamToCheck 0)
      (LocalVariables|SetLcl_playersInThisTeam 0 :!label _label_3)
      (for _array_element_5 (Variables|Default|GetAll_TeamIDs)
        (if (== _array_element_5 (LocalVariables|GetLcl_TeamToCheck))
          (Math|Integer|IncrementInt (LocalVariables|GetLcl_playersInThisTeam))))
      (if (< (LocalVariables|GetLcl_playersInThisTeam) (Variables|Default|GetMaxTeamSize))
        (Utilities|Array|SetArrayElem (Variables|Default|GetAll_TeamIDs) (Utilities|Array|FindItem (Variables|Default|GetAll_TeamIDs) _array_index_2) (LocalVariables|GetLcl_TeamToCheck) true)
        (LocalVariables|SetLcl_IDsOverWrite true)
        (Utilities|Array|SetArrayElem (LocalVariables|GetLcl_TeamCounts) _array_index_2 (- (Utilities|Array|Get(acopy) (LocalVariables|GetLcl_TeamCounts) _array_index_2) 1))
        (goto _label_2)
        (else
          (Math|Integer|IncrementInt (LocalVariables|GetLcl_TeamToCheck)
            (:%20%20
              (if (not (== (LocalVariables|GetLcl_TeamToCheck) (Variables|Default|GetNrOfTeams)))
                (goto _label_3))))))))
  (return (LocalVariables|GetLcl_IDsOverWrite)))

(fn MakeTeams
  (bind _lcl_playerlevels (LocalVariables|GetLcl_PlayerLevels))
  (bind (_indexofmaxvalue _maxvalue) (Math|Integer|MaxOfIntArray _lcl_playerlevels))
  (for (_array_element _array_index) (Variables|Default|GetAll_PlayerProfiles)
    (Utilities|Array|SetArrayElem (LocalVariables|GetLcl_PlayerLevels) _array_index (Utilities|Struct|BreakS_PlayerProfile _array_element) true))
  (LocalVariables|SetLcl_IndexWithMaxValue _indexofmaxvalue :!label _label)
  (if (!= _maxvalue 0)
    (Utilities|Array|SetArrayElem (Variables|Default|GetAll_TeamIDs) (LocalVariables|GetLcl_IndexWithMaxValue) (LocalVariables|GetLcl_AddPlayerToTeam))
    (Utilities|Array|SetArrayElem (LocalVariables|GetLcl_PlayerLevels) (LocalVariables|GetLcl_IndexWithMaxValue) 0)
    (Math|Integer|IncrementInt (LocalVariables|GetLcl_AddPlayerToTeam)
      (:%20%20
        (if (== (LocalVariables|GetLcl_AddPlayerToTeam) (Variables|Default|GetNrOfTeams))
          (LocalVariables|SetLcl_AddPlayerToTeam 0)
          (goto _label)
          (else
            (goto _label)))))))

(fn TransferTeamIDs
  (for (_array_element _array_index) (Variables|Default|GetAll_ConnectedPlayers)
    (Default|SaveTeamID _array_element (Utilities|Array|Get(acopy) (Variables|Default|GetAll_TeamIDs) _array_index))))

(fn DisdableAllLobies
  (for _array_element (Variables|Default|GetAll_ConnectedPlayers)
    (Default|DisableLobbyMenu _array_element)))

(fn SetLobbyCharacterModelandSkin
  (params (BP_LobbyCharacter :type Lobby%20Character%20BP%20Object%20Reference) (CharRowName :type Name) (ModelName :type Name%20%28by%20ref%29) (SkinName :type Name))
  (bind _returnvalue (Utilities|GetDataTableRow "/Game/Player/CharCustomisationm_Table.CharCustomisationm_Table" CharRowName)
    (:then
      (Default|MCSetCharMesh BP_LobbyCharacter (.Model (Utilities|Struct|BreakS_ModelAndSkins (.Value (Utilities|Map|Find (.ModelsAndSkins (Utilities|Struct|BreakS_CharCustomisation _returnvalue)) ModelName)))))
      (Default|MCPlayMeshAnim BP_LobbyCharacter (.LobbyAnimation (Utilities|Struct|BreakS_ModelAndSkins (.Value (Utilities|Map|Find (.ModelsAndSkins (Utilities|Struct|BreakS_CharCustomisation _returnvalue)) ModelName)))))
      (if (.Use_Skin0 (Utilities|Struct|BreakS_ModelAndSkins (.Value (Utilities|Map|Find (.ModelsAndSkins (Utilities|Struct|BreakS_CharCustomisation _returnvalue)) ModelName))))
        (Default|MCSetSkinMaterial BP_LobbyCharacter (.Skin0_MaterialSlot (Utilities|Struct|BreakS_ModelAndSkins (.Value (Utilities|Map|Find (.ModelsAndSkins (Utilities|Struct|BreakS_CharCustomisation _returnvalue)) ModelName)))) (.Value (Utilities|Map|Find (.Skin0_Skins (Utilities|Struct|BreakS_ModelAndSkins (.Value (Utilities|Map|Find (.ModelsAndSkins (Utilities|Struct|BreakS_CharCustomisation _returnvalue)) ModelName)))) SkinName))))
      (if (.Use_Skin1 (Utilities|Struct|BreakS_ModelAndSkins (.Value (Utilities|Map|Find (.ModelsAndSkins (Utilities|Struct|BreakS_CharCustomisation _returnvalue)) ModelName))))
        (Default|MCSetSkinMaterial BP_LobbyCharacter (.Skin1_MaterialSlot (Utilities|Struct|BreakS_ModelAndSkins (.Value (Utilities|Map|Find (.ModelsAndSkins (Utilities|Struct|BreakS_CharCustomisation _returnvalue)) ModelName)))) (.Value (Utilities|Map|Find (.Skin1_Skins (Utilities|Struct|BreakS_ModelAndSkins (.Value (Utilities|Map|Find (.ModelsAndSkins (Utilities|Struct|BreakS_CharCustomisation _returnvalue)) ModelName)))) SkinName)))))))

(fn GMTDMOverrideLobbyCharacter
  (params (UseOverride :type Boolean) (PlayerController :type BP%20Menu%20Controller%20Object%20Reference))
  (LocalVariables|SetLcl_PlayerIndex (Utilities|Array|FindItem (Variables|Default|GetAll_ConnectedPlayers) PlayerController))
  (if UseOverride
    (switch int (Utilities|Array|Get(acopy) (Variables|Default|GetAll_TeamIDs) (LocalVariables|GetLcl_PlayerIndex))
      (:0
        (LocalVariables|SetLcl_CharRowName "Player_Blue")
        (LocalVariables|SetLcl_ModelName (.ModelName (Utilities|Struct|BreakS_PlayerProfile (Utilities|Array|Get(acopy) (Variables|Default|GetAll_PlayerProfiles) (LocalVariables|GetLcl_PlayerIndex)))))
        (LocalVariables|SetLcl_SkinName "Default"))
      (:1
        (LocalVariables|SetLcl_CharRowName "Player_Green")
        (LocalVariables|SetLcl_ModelName (.ModelName (Utilities|Struct|BreakS_PlayerProfile (Utilities|Array|Get(acopy) (Variables|Default|GetAll_PlayerProfiles) (LocalVariables|GetLcl_PlayerIndex)))))
        (LocalVariables|SetLcl_SkinName "Default"))
      (:2
        (LocalVariables|SetLcl_CharRowName "Player_Red")
        (LocalVariables|SetLcl_ModelName (.ModelName (Utilities|Struct|BreakS_PlayerProfile (Utilities|Array|Get(acopy) (Variables|Default|GetAll_PlayerProfiles) (LocalVariables|GetLcl_PlayerIndex)))))
        (LocalVariables|SetLcl_SkinName "Default"))
      (:3
        (LocalVariables|SetLcl_CharRowName "Player_Yellow")
        (LocalVariables|SetLcl_ModelName (.ModelName (Utilities|Struct|BreakS_PlayerProfile (Utilities|Array|Get(acopy) (Variables|Default|GetAll_PlayerProfiles) (LocalVariables|GetLcl_PlayerIndex)))))
        (LocalVariables|SetLcl_SkinName "Default")))
    (CallFunction|SetLobbyCharacterModelandSkin (Variables|/Game/Framework/BP_MenuController.BP_MenuController_C|GetLobbyCharacter_BP PlayerController) (LocalVariables|GetLcl_CharRowName) (LocalVariables|GetLcl_ModelName) (LocalVariables|GetLcl_SkinName))
    (else
      (CallFunction|UpdateSelectedCharacter (LocalVariables|GetLcl_PlayerIndex)))))