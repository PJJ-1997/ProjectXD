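; Player controller for the multiplayer shooter, managing player profile, match UI, and respawn or spectate after death.
; Loads the saved profile, sends it to the server and saves XP changes after a retriggerable delay.
; Polls until game state, player state and profile are ready.
; Game mode sets respawn, spectate and team flags; events drive HUD, scoreboard, death and game-over widgets, while the controller's own spectator target-cycling functions are disconnected.
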(event Custom|EnableAllInput
  (Input|EnableInput (Pawn|GetControlledPawn) self))

(event Custom|GameStartCountdown
  (Default|GameStartCountdown (Variables|Default|GetWB_IngameHUD)))

(event Custom|ShowSpectatorControls
  (Default|ShowSpectatorControls (Variables|Default|GetWB_PlayerDiedMenu) true)
  (Variables|Default|SetbShowMouseCursor false)
  (Input|SetInputModeGameOnly self false))

(event Custom|UpdateHUD_SpectatorPlayerName
  (params (PlayerName :type Text))
  (Default|UpdateSpectatorName (Variables|Default|GetWB_PlayerDiedMenu) PlayerName))

(event Custom|Svr_GetSpectatorPlayerName
  (params (SpectatorTarget :type BP%20C%20Player%20Base%20Object%20Reference))
  (CallFunction|UpdateHUDSpectatorPlayerName (.PlayerName (Utilities|Struct|BreakS_PlayerProfile (Variables|BP_ShooterPlayerController_C|GetS_PlayerProfile (Variables|/Game/Player/BP_CPlayer_Base.BP_CPlayer_Base_C|GetBP_SHooterPlayerController SpectatorTarget))))))

(event Custom|Svr_IsRespawnEnabled
  (bind _asbp_shooter_game_mode (Utilities|Casting|CastToBP_ShooterGameMode (Game|GetGameMode)))
  (switch Utilities|FlowControl|Switch|SwitchonE_GameModes (Variables|/Game/Framework/BP_ShooterGameMode.BP_ShooterGameMode_C|GetGameMode _asbp_shooter_game_mode)
    (:NewEnumerator0
      (Variables|Default|SetIsRespawnEnabled false)
      (Variables|Default|SetIsSpectatingEnabled true)
      (Variables|Default|SetIsModeFFA false)
      (Variables|Default|SetIsModeTDM false))
    (:NewEnumerator1
      (Variables|Default|SetIsRespawnEnabled true)
      (Variables|Default|SetIsSpectatingEnabled false)
      (Variables|Default|SetIsModeFFA true)
      (Variables|Default|SetIsModeTDM false))
    (:NewEnumerator2
      (Variables|Default|SetIsRespawnEnabled true)
      (Variables|Default|SetIsSpectatingEnabled true)
      (Variables|Default|SetIsModeFFA false)
      (Variables|Default|SetIsModeTDM true))))

(event Custom|Loadprofile
  (bind _asbp_shooter_game_instance (Utilities|Casting|CastToBP_ShooterGameInstance (Game|GetGameInstance)))
  (Variables|Default|SetPlayer%20Profile%20Slot (Variables|/Game/Framework/BP_ShooterGameInstance.BP_ShooterGameInstance_C|GetPlayerProfile_Slot _asbp_shooter_game_instance))
  (bind _returnvalue (SaveGame|LoadGamefromSlot (Variables|Default|GetPlayer%20Profile%20Slot)))
  (bind _assg_player_profile (Utilities|Casting|CastToSG_PlayerProfile _returnvalue))
  (Variables|Default|SetAs%20SG%20Player%20Profile _assg_player_profile)
  (Networking|SwitchHasAuthority
    (:Authority
      (bind _output_get (Variables|Default|SetS_PlayerProfile (Variables|/Game/SavedData/SG_PlayerProfile.SG_PlayerProfile_C|GetPlayerProfile _assg_player_profile)))
      (Variables|Default|SetTeamID (Utilities|Struct|BreakS_PlayerProfile _output_get))
      (if (Variables|Default|GetIsPlayerStateReady) :!label _label
        (Variables|/Game/Framework/BP_ShooterPlayerstate.BP_ShooterPlayerstate_C|SetTeamID (Variables|Default|GetBP_ShooterPlayerState) (Variables|Default|GetTeamID))
        (Variables|Default|SetIsProfileLoaded true)
        (else
          (Utilities|FlowControl|DelayUntilNextTick)
          (goto _label))))
    (:Remote
      ;[1 1 1] Server_PlayerProfile
      (CallFunction|SvrSetPlayerProfile (Variables|/Game/SavedData/SG_PlayerProfile.SG_PlayerProfile_C|GetPlayerProfile _assg_player_profile)))))

(event Custom|Svr_charBeginPlay
  (bind _asbp_cplayer_base (Utilities|Casting|CastToBP_CPlayer_Base (Pawn|GetControlledPawn)))
  (Default|MCBeginPlay _asbp_cplayer_base))

(event Custom|ShowGameOverScreen
  (params (WavesSurvived :type Integer) (IsWinner :type Boolean) (IsScoreLimit :type Boolean) (IsTimeLimit :type Boolean) (GameMode :type E_GameModes%20Enum :default "NewEnumerator0") (WinningTeamID :type Integer))
  (Viewport|RemoveAllWidgets)
  (bind _returnvalue (UserInterface|CreateWidget "/Game/Widgets/WB_GameOverMenu.WB_GameOverMenu_C" self WavesSurvived IsWinner IsScoreLimit IsTimeLimit GameMode WinningTeamID))
  (UserInterface|Viewport|AddtoViewport _returnvalue 0))

(event Custom|OnControllerSpawned
  (if (Variables|Default|GetIsGameStateReady) :!label _label
    _
    (else
      (bind _asshooter_game_state (Utilities|Casting|CastToShooterGameState (Game|GetGameState))
        (:then
          (Variables|Default|SetBP_ShooterGameState _asshooter_game_state)
          (Variables|Default|SetIsGameStateReady true))
        (:CastFailed
          _))))
  (if (Variables|Default|GetIsPlayerStateReady)
    _
    (else
      (bind _asbp_shooter_playerstate (Utilities|Casting|CastToBP_ShooterPlayerstate (Variables|Default|GetPlayerState))
        (:then
          (Variables|Default|SetBP_ShooterPlayerState _asbp_shooter_playerstate)
          (Variables|Default|SetIsPlayerStateReady true))
        (:CastFailed
          _))))
  (if (Math|Boolean|ANDBoolean (Variables|Default|GetIsProfileLoaded) (Variables|Default|GetIsGameStateReady) (Variables|Default|GetIsPlayerStateReady))
    ;[1 1 1] Everything is loaded
    (Variables|Default|SetIsPlayerReady true)
    (else
      (Utilities|FlowControl|Delay 0.1)
      (goto _label))))

(event Custom|UnHide_IngameHUD
  (Widget|SetVisibility (Variables|Default|GetWB_IngameHUD) "Visible"))

(event Custom|HUD_StartMatch_PvP
  (Default|GMPvPStartMatch (Variables|Default|GetWB_IngameHUD)))

(event Custom|HUD_SetupMatchTimer
  (params (TimeLeftSec :type Integer))
  (bind _wb_ingamehud (Variables|Default|GetWB_IngameHUD))
  (Widget|SetVisibility (Variables|/Game/Widgets/WB_IngameHUD.WB_IngameHUD_C|GetText_MatchDuration _wb_ingamehud) "Visible")
  (Default|UpdMatchTimer _wb_ingamehud TimeLeftSec))

(event Custom|UI_ShowKillMessage
  (params (IsKiller :type Boolean) (VictimName :type Text) (KillerName :type Text) (KillXP :type Integer))
  (bind _wb_ingamehud (Variables|Default|GetWB_IngameHUD))
  (Utilities|IsValid _wb_ingamehud
    (:Is%20Valid
      (Default|ShowKillMessage _wb_ingamehud IsKiller VictimName KillerName KillXP))))

(event Custom|Controller_DisableInput
  (Input|DisableInput (Pawn|GetControlledPawn) self))

(event Custom|Client_ToggleScoreboard
  (params (Newvisibility :type Boolean))
  (CallFunction|UIToggleScoreBoard Newvisibility))

(event Custom|UI_UpdateNewsFeed
  (params (NewsfeedLine :type Text))
  (bind _wb_ingamehud (Variables|Default|GetWB_IngameHUD))
  (Utilities|IsValid _wb_ingamehud
    (:Is%20Valid
      (Default|AddLinetoNewsfeed _wb_ingamehud NewsfeedLine))))

(event Custom|SetSpawnRotation
  (params (New%20Rotation%20Z%20%28Yaw%29 :type Float%20%28single-precision%29))
  (Pawn|SetControlRotation (Math|Rotator|MakeRotator 0.0 0.0 New%20Rotation%20Z%20%28Yaw%29)))

(event Custom|HUD_UpdateScoreboard
  (bind _wb_scoreboard (Variables|Default|GetWB_Scoreboard))
  (Utilities|IsValid _wb_scoreboard
    (:Is%20Valid
      (if (UserInterface|Viewport|IsinViewport _wb_scoreboard)
        (Default|UpdateScoreboard _wb_scoreboard)))))

(event Custom|EndClientSession
  (bind _asbp_shooter_game_instance (Utilities|Casting|CastToBP_ShooterGameInstance (Game|GetGameInstance)))
  (Variables|/Game/Framework/BP_ShooterGameInstance.BP_ShooterGameInstance_C|SetMP_IsPAuseMenuVisible _asbp_shooter_game_instance false)
  (|DestroySession self
    (:OnSuccess
      (Game|OpenLevel(byName) "MainMenu_Map"))))

(event Custom|Svr_SetPlayerProfile
  (params (S_PlayerProfile :type S%20Player%20Profile%20Structure))
  (Variables|Default|SetS_PlayerProfile S_PlayerProfile)
  (Variables|Default|SetTeamID (Utilities|Struct|BreakS_PlayerProfile (stale Custom|Loadprofile _output_get)))
  (if (Variables|Default|GetIsPlayerStateReady) :!label _label
    (Variables|/Game/Framework/BP_ShooterPlayerstate.BP_ShooterPlayerstate_C|SetTeamID (Variables|Default|GetBP_ShooterPlayerState) (Variables|Default|GetTeamID))
    (Variables|Default|SetIsProfileLoaded true)
    (else
      (Utilities|FlowControl|DelayUntilNextTick)
      (goto _label))))

(event Custom|Save_XPandLevel
  (bind _as_sg_player_profile (Variables|Default|GetAs%20SG%20Player%20Profile))
  ;[1 1 1] .5 -> 1
  (Utilities|FlowControl|RetriggerableDelay 0.5)
  (Variables|/Game/SavedData/SG_PlayerProfile.SG_PlayerProfile_C|SetPlayerProfile _as_sg_player_profile (Variables|Default|GetS_PlayerProfile))
  (SaveGame|SaveGametoSlot _as_sg_player_profile (Variables|Default|GetPlayer%20Profile%20Slot)))

(event Custom|Client_HUD_StartNewWave
  (params (WaveNumber :type Integer))
  (Default|GMEWStartNewWave (Variables|Default|GetWB_IngameHUD) WaveNumber))

(event Custom|RespawnAfterDeath
  (Variables|Default|SetIsSpectating false)
  (bind _asbp_shooter_game_mode (Utilities|Casting|CastToBP_ShooterGameMode (Game|GetGameMode)))
  (Default|RespawnAfterDying _asbp_shooter_game_mode self))

(event Custom|MC_BeginPlay
  (bind _returnvalue (Pawn|GetControlledPawn))
  (if (Pawn|IsLocalPlayerController)
    (if (Variables|Default|GetIsSpectating)
      (Utilities|IsValid _returnvalue :!label _label
        (:Is%20Valid
          (bind _asbp_spectator (Utilities|Casting|CastToBP_Spectator _returnvalue))
          (Variables|Default|SetBP_Spectator _asbp_spectator))
        (:Is%20Not%20Valid
          (Utilities|FlowControl|DelayUntilNextTick)
          (goto _label)))
      (else
        (Viewport|RemoveAllWidgets)
        (Input|SetInputModeGameOnly self false)
        (Variables|Default|SetbShowMouseCursor false)
        (CallFunction|UIShowIngameHUD)
        (CallFunction|SvrIsRespawnEnabled)
        (Networking|SwitchHasAuthority
          (:Authority
            (bind _asbp_cplayer_base (Utilities|Casting|CastToBP_CPlayer_Base (Pawn|GetControlledPawn)))
            (Default|MCBeginPlay _asbp_cplayer_base))
          (:Remote
            (CallFunction|SvrCharBeginPlay)))))
    (else
      (Actor|Tick|SetActorTickEnabled false))))

(event Custom|SpectateAfterDeath
  (Variables|Default|SetIsSpectating true)
  (bind _asbp_shooter_game_mode (Utilities|Casting|CastToBP_ShooterGameMode (Game|GetGameMode)))
  (Default|SpawnSpectatorAfterDying _asbp_shooter_game_mode self))

(event EventTick
  (params (DeltaSeconds :type Float%20%28single-precision%29))
  (bind _returnvalue (Pawn|GetControlRotation :!class /Script/Engine.Controller))
  (if (Variables|Default|GetIsSpectating)
    (bind _bp_spectator (Variables|Default|GetBP_Spectator)
      (:then
        (Variables|/Game/Player/BP_Spectator.BP_Spectator_C|GetAttachedPlayer _bp_spectator
          (:then
            (Pawn|SetControlRotation (Math|Rotator|MakeRotator (.roll _returnvalue) (.pitch _returnvalue) 0.0)))
          (:else)))
      (:else))))

(event EventPossess
  (params (PossessedPawn :type Pawn%20Object%20Reference))
  (CallFunction|MCBeginPlay))

(fn ConstructionScript)

(fn UIShowIngameHUD
  (Utilities|IsValid (Variables|Default|GetWB_IngameHUD)
    (:Is%20Valid
      _)
    (:Is%20Not%20Valid
      (bind _returnvalue (UserInterface|CreateWidget "/Game/Widgets/WB_IngameHUD.WB_IngameHUD_C" self))
      (bind _output_get (Variables|Default|SetWB_IngameHUD _returnvalue))))
  (UserInterface|Viewport|AddtoViewport _output_get 0)
  (return))

(fn UIShowDiedMenu
  (bind _wb_ingamehud (Variables|Default|GetWB_IngameHUD))
  (bind _wb_ingamehud_2 (Variables|Default|GetWB_IngameHUD))
  (if (not (Variables|Default|GetIsGameOver))
    (bind _outactors (Actor|GetAllActorsOfClass "/Game/Player/BP_CPlayer_Base.BP_CPlayer_Base_C"))
    (for _array_element _outactors
      (if (not (Variables|/Game/Player/BP_CPlayer_Base.BP_CPlayer_Base_C|GetIsAlive _array_element))
        (Math|Integer|IncrementInt (LocalVariables|GetLcl_DeadPlayers))))
    (if (== (Utilities|Array|Length _outactors) (LocalVariables|GetLcl_DeadPlayers))
      (Utilities|IsValid _wb_ingamehud_2
        (:Is%20Valid
          (Widget|RemovefromParent _wb_ingamehud_2)))
      (else
        (Utilities|IsValid _wb_ingamehud
          (:Is%20Valid
            (Widget|RemovefromParent _wb_ingamehud)
            (Utilities|IsValid (Variables|Default|GetWB_PlayerDiedMenu)
              (:Is%20Valid
                _)
              (:Is%20Not%20Valid
                (bind _returnvalue (UserInterface|CreateWidget "/Game/Widgets/WB_PlayerDiedMenu.WB_PlayerDiedMenu_C" self))
                (Variables|Default|SetWB_PlayerDiedMenu _returnvalue)))
            (UserInterface|Viewport|AddtoViewport (Variables|Default|GetWB_PlayerDiedMenu) 0)
            (Input|SetInputModeUIOnly self 0 "DoNotLock" false)
            (Variables|Default|SetbShowMouseCursor true)))))
    (return)))

(fn SpectatorUpdateTargets)

(fn SpectatorStartSpectateTarget
  (params (Previous :type Boolean)))

(fn UIToggleScoreBoard
  (params (Newvisibility :type Boolean))
  (if Newvisibility
    (Utilities|IsValid (Variables|Default|GetWB_Scoreboard)
      (:Is%20Valid
        _)
      (:Is%20Not%20Valid
        (bind _returnvalue (UserInterface|CreateWidget "/Game/Widgets/WB_Scoreboard.WB_Scoreboard_C" self))
        (Variables|Default|SetWB_Scoreboard _returnvalue)))
    (UserInterface|Viewport|AddtoViewport (Variables|Default|GetWB_Scoreboard) 0)
    (else
      (Utilities|IsValid (Variables|Default|GetWB_Scoreboard)
        (:Is%20Valid
          (Widget|RemovefromParent (Variables|Default|GetWB_Scoreboard)))
        (:Is%20Not%20Valid
          _))))
  (return))