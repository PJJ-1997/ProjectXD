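; Player state for the shooter that holds each player's profile and display name.
; On BeginPlay, the server caches the owning shooter controller and polls every tick until its profile is loaded, then copies the profile and sets the player name.
; CopyProperties passes the profile, but not the separate name variable, to a replacement player state.
; The name has a RepNotify function, which is empty.
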(event EventBeginPlay
  (if (Networking|IsServer)
    (bind _asbp_shooter_player_controller (Utilities|Casting|CastToBP_ShooterPlayerController (Game|GetPlayerController)))
    (bind _output_get (Variables|Default|SetBP_SHooterPlayerController _asbp_shooter_player_controller))
    (if (Variables|/Game/Framework/BP_ShooterPlayerController.BP_ShooterPlayerController_C|GetIsProfileLoaded _output_get) :!label _label
      (bind _output_get_2 (Variables|Default|SetS_PlayerProfile (Variables|/Game/Framework/BP_ShooterPlayerController.BP_ShooterPlayerController_C|GetS_PlayerProfile _output_get)))
      (Variables|Default|SetMy_PlayerName (.PlayerName (Utilities|Struct|BreakS_PlayerProfile _output_get_2)))
      (else
        (Utilities|FlowControl|DelayUntilNextTick)
        (goto _label)))))

(event EventCopyProperties
  (params (NewPlayerState :type Player%20State%20Object%20Reference))
  (bind _asbp_shooter_playerstate (Utilities|Casting|CastToBP_ShooterPlayerstate NewPlayerState))
  (Variables|BP_ShooterPlayerstate_C|SetS_PlayerProfile _asbp_shooter_playerstate (Variables|Default|GetS_PlayerProfile)))

(fn ConstructionScript)

(fn OnRepMyPlayerName)