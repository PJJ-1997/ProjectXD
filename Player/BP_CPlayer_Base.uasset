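; Base player character for the multiplayer shooter, handling data-table stats and skins, firing, damage, death, XP and HUD hooks.
; Held fire repeats a camera line trace, and hits go through damage interfaces, awarding XP for kills on that path.
; Incoming damage splits into AI and FFA/TDM team-checked PvP paths, using separate health variables.
; Death plays a montage, blends to a death camera and notifies the game mode; hit montages are empty.
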(event Custom|DisableAllInput
  (params (PlayerController :type Player%20Controller%20Object%20Reference))
  (Input|DisableInput PlayerController))

(event Custom|MC_BeginPlay
  (bind _bp_shooterplayercontroller (Variables|Default|GetBP_ShooterPlayerController))
  ;[1 1 1] Customisation
  (CallFunction|SetModelandSkin)
  ;[1 1 1] 경험치
  (Default|XPComponentInit (Variables|Default|GetBP_XP_Component))
  (if (Pawn|IsLocallyControlled)
    ;[1 1 1] BP에서 만든 플레이어 캐릭터들의 체력 상태들 표시 / 없어도 된다.
    (Development|PrintString (Utilities|String|ToString(Text) (Utilities|Text|FormatText " 
Health: {a} 
Strength: {b} 
Stamina: {c}" (Variables|Default|GetHealth) (Variables|Default|GetBP_Stamina) (Variables|Default|GetBP_Strength))) true true "(R=0.000000,G=0.660000,B=1.000000,A=1.000000)" 15.0)
    (bind _output_get (Variables|Default|SetWB%20Ingame%20HUD (Variables|/Game/Framework/BP_ShooterPlayerController.BP_ShooterPlayerController_C|GetWB_IngameHUD (Variables|Default|GetBP_SHooterPlayerController))))
    (Default|UpdateHealth _output_get (Variables|Default|GetHealth) false))
  (if (Networking|IsServer)
    (Variables|Default|SetIsModeFFA (Variables|/Game/Framework/BP_ShooterPlayerController.BP_ShooterPlayerController_C|GetIsModeFFA _bp_shooterplayercontroller))
    (Variables|Default|SetIsModeTDM (Variables|/Game/Framework/BP_ShooterPlayerController.BP_ShooterPlayerController_C|GetIsModeTDM _bp_shooterplayercontroller))
    (Variables|Default|SetTeam%20ID (Variables|/Game/Framework/BP_ShooterPlayerController.BP_ShooterPlayerController_C|GetTeamID _bp_shooterplayercontroller))
    (bind _asbp_shooter_game_mode (Utilities|Casting|CastToBP_ShooterGameMode (Game|GetGameMode)))
    (Variables|Default|SetRespawnDelay (Math|Conversions|ToFloat(Integer) (Variables|/Game/Framework/BP_ShooterGameMode.BP_ShooterGameMode_C|GetRespawnDelay _asbp_shooter_game_mode)))))

(event Custom|Client_BeginFire
  (Class|CWeaponComponent|BeginFire (Variables|Default|GetWeapon)))

(event Custom|Svr_EndFire
  ;[1 1 1] 임시로
  (CallFunction|ClientEndFire))

(event Custom|MC_AIMeleeImpact
  (params (Location :type Vector) (Normal :type Vector) (MontageToPlay :type Anim%20Montage%20Object%20Reference))
  (Effects|SpawnEmitteratLocation 0 Location (Math|Conversions|RotationFromXVector Normal))
  (Animation|Montage|PlayMontage (Variables|Character|GetMesh) MontageToPlay))

(event Custom|HUD_CreateDaamageIndicator
  (params (AttackLocation :type Vector))
  (Default|CreateDamageIndicator (Variables|Default|GetWB%20Ingame%20HUD) AttackLocation))

(event Custom|ClientUpdateHUD_Health
  (params (NewHealth :type Float%20%28double-precision%29) (Melee_DamageAnim :type Boolean))
  (Default|UpdateHealth (Variables|Default|GetWB%20Ingame%20HUD) NewHealth Melee_DamageAnim))

(event Custom|Start_Ragdoll
  ;[1 1 1] Diying Ragdoll 사용 x
)

(event Custom|Die
  (params (RespawnDelay :type Float%20%28single-precision%29))
  (bind _bp_shooterplayercontroller (Variables|Default|GetBP_SHooterPlayerController))
  (Input|DisableInput _bp_shooterplayercontroller)
  (Game|Player|SetViewTargetwithBlend _bp_shooterplayercontroller (Variables|/Script/Engine.ChildActorComponent|GetChildActor (Variables|Default|GetCameraTargetDeath)) 2.0 "VTBlend_Linear" 0.0 false)
  (Actor|Tick|SetActorTickEnabled false)
  (Networking|SwitchHasAuthority
    (:Authority
      (Variables|/Script/Engine.CharacterMovementComponent|SetbUseControllerDesiredRotation (Variables|Character|GetCharacterMovement) false))
    (:Remote
      (CallFunction|SvrSetControllerDesRotation false)
      (Variables|/Script/Engine.CharacterMovementComponent|SetbUseControllerDesiredRotation (Variables|Character|GetCharacterMovement) false)))
  (Utilities|FlowControl|Delay RespawnDelay)
  (Default|UIShowDiedMenu _bp_shooterplayercontroller))

(event Custom|Svr_SetControllerDesRotation
  (params (Use%20Controller%20Desired%20Rotation :type Boolean))
  (Variables|/Script/Engine.CharacterMovementComponent|SetbUseControllerDesiredRotation (Variables|Character|GetCharacterMovement) Use%20Controller%20Desired%20Rotation))

(event Custom|Svr_BeginFire
  (bind _camera (Variables|Default|GetCamera))
  (bind _returnvalue (Transformation|GetWorldTransform _camera))
  (bind _returnvalue_2 (Math|Vector|GetForwardVector (.rotation _returnvalue)))
  ;[1 1 1] 임시로
  (if (not (Class|CWeaponComponent|IsUnarmedMode (Variables|Default|GetWeapon)))
    (CallFunction|ClientBeginFire)
    (Utilities|FlowControl|Delay 0.1)
    (bind _outhit (Collision|LineTraceByChannel (+ (.location _returnvalue) (* _returnvalue_2 300)) (+ (.location _returnvalue) (* _returnvalue_2 100000)) "TraceTypeQuery3" false 0 "None"))
    (CallFunction|SvrProcessHit _outhit)
    (Development|PrintString "Hit" true true "(R=1.000000,G=0.000000,B=0.018187,A=1.000000)" 5.0)))

(event Custom|Client_EndFire
  (Class|CWeaponComponent|EndFire (Variables|Default|GetWeapon)))

(event EventAddXP
  (params (XP_Amount :type Integer))
  (Default|ComponentAddXP (Variables|Default|GetBP_XP_Component) XP_Amount)
  (Development|PrintString (Utilities|String|ToString(Integer) XP_Amount)))

(event EventPlayerTakeDamage
  (params (Attacker :type Actor%20Object%20Reference) (HitResult :type Hit%20Result%20Structure) (Amount :type Float%20%28double-precision%29) (IsPvPDamage :type Boolean) (TeamID :type Integer))
  (if IsPvPDamage
    (CallFunction|TakePvPDamage Attacker HitResult Amount TeamID)
    (else
      (CallFunction|TakeAIDamage Attacker HitResult Amount))))

(event EventUnpossessed
  (params (OldController :type Controller%20Object%20Reference))
  (Actor|DestroyActor))

(event EventPossessed
  (params (NewController :type Controller%20Object%20Reference))
  (bind _asbp_shooter_player_controller (Utilities|Casting|CastToBP_ShooterPlayerController NewController))
  (Variables|Default|SetBP_SHooterPlayerController _asbp_shooter_player_controller)
  (if (Variables|Default|GetDeathRespawn)
    (Variables|Default|SetDeathRespawn false)
    (else
      (CallFunction|DisableAllInput (Variables|Default|GetBP_SHooterPlayerController)))))

(event Input|ActionEvents|InputActionToggle_Scoreboard
  (params (Key :type Key%20Structure :default "None"))
  (bind _bp_shooterplayercontroller (Variables|Default|GetBP_SHooterPlayerController))
  (:Pressed
    (Default|UIToggleScoreBoard _bp_shooterplayercontroller true))
  (:Released
    (Default|UIToggleScoreBoard _bp_shooterplayercontroller false)))

(event Input|ActionEvents|InputActionFire
  (params (Key :type Key%20Structure :default "None"))
  (:Pressed
    (bind _returnvalue (Utilities|Time|SetTimerbyFunctionName 0 "Svr_BeginFire" 0.1 true))
    (CallFunction|SvrBeginFire))
  (:Released
    (Utilities|Time|ClearandInvalidateTimerbyHandle _returnvalue)
    (CallFunction|SvrEndFire)))

(event Input|ActionEvents|InputActionPauseGame
  (params (Key :type Key%20Structure :default "None"))
  (:Pressed
    (bind _asbp_shooter_game_instance (Utilities|Casting|CastToBP_ShooterGameInstance (Game|GetGameInstance)))
    (bind _isgamepausedresult (Default|TogglePauseGame _asbp_shooter_game_instance))
    (if _isgamepausedresult
      (Widget|SetVisibility (Variables|Default|GetWB%20Ingame%20HUD) "Hidden"))))

(fn ConstructionScript
  (Networking|SwitchHasAuthority
    (:Authority
      (bind _returnvalue (Utilities|GetDataTableRow "/Game/Player/CharacterInfo_Table.CharacterInfo_Table" (Variables|Default|GetCharRowName))
        (:then
          (Variables|Default|SetHealth (.Health (Utilities|Struct|BreakS_CharacterInfo _returnvalue)))
          (Variables|Default|SetBP_Stamina (.Stamina (Utilities|Struct|BreakS_CharacterInfo _returnvalue)))
          (Variables|Default|SetBP_Strength (.Strength (Utilities|Struct|BreakS_CharacterInfo _returnvalue))))))))

(fn SetModelandSkin
  (bind _mesh (Variables|Character|GetMesh))
  (bind _skinname (Variables|Default|GetSkinName))
  (bind _returnvalue (Utilities|GetDataTableRow "/Game/Player/CharCustomisationm_Table.CharCustomisationm_Table" (Variables|Default|GetCharRowName))
    (:then
      (Components|SkinnedMesh|SetSkinnedAssetandUpdate _mesh (.Model (Utilities|Struct|BreakS_ModelAndSkins (.Value (Utilities|Map|Find (.ModelsAndSkins (Utilities|Struct|BreakS_CharCustomisation _returnvalue)) (Variables|Default|GetModelName))))) true)
      (if (.Use_Skin0 (Utilities|Struct|BreakS_ModelAndSkins (.Value (Utilities|Map|Find (.ModelsAndSkins (Utilities|Struct|BreakS_CharCustomisation _returnvalue)) (Variables|Default|GetModelName)))))
        (Rendering|Material|SetMaterial _mesh (.Skin0_MaterialSlot (Utilities|Struct|BreakS_ModelAndSkins (.Value (Utilities|Map|Find (.ModelsAndSkins (Utilities|Struct|BreakS_CharCustomisation _returnvalue)) (Variables|Default|GetModelName))))) (.Value (Utilities|Map|Find (.Skin0_Skins (Utilities|Struct|BreakS_ModelAndSkins (.Value (Utilities|Map|Find (.ModelsAndSkins (Utilities|Struct|BreakS_CharCustomisation _returnvalue)) (Variables|Default|GetModelName))))) _skinname))))
      (if (.Use_Skin1 (Utilities|Struct|BreakS_ModelAndSkins (.Value (Utilities|Map|Find (.ModelsAndSkins (Utilities|Struct|BreakS_CharCustomisation _returnvalue)) (Variables|Default|GetModelName)))))
        (Rendering|Material|SetMaterial _mesh (.Skin1_MaterialSlot (Utilities|Struct|BreakS_ModelAndSkins (.Value (Utilities|Map|Find (.ModelsAndSkins (Utilities|Struct|BreakS_CharCustomisation _returnvalue)) (Variables|Default|GetModelName))))) (.Value (Utilities|Map|Find (.Skin1_Skins (Utilities|Struct|BreakS_ModelAndSkins (.Value (Utilities|Map|Find (.ModelsAndSkins (Utilities|Struct|BreakS_CharCustomisation _returnvalue)) (Variables|Default|GetModelName))))) _skinname)))))))

(fn SvrProcessHit
  (params (HitResult :type Hit%20Result%20Structure))
  (bind (_bblockinghit _binitialoverlap _time _distance _location _impactpoint _normal _impactnormal _physmat _hitactor _hitcomponent _hitbonename) (Collision|BreakHitResult HitResult))
  (if (and _bblockinghit (Utilities|DoesObjectImplementInterface _hitactor "/Game/Framework/Interface/BPI_Damage_Interface.BPI_Damage_Interface_C"))
    (bind (_isdead _xp _isvalidhit) (Class|BPIDamageInterface|TakeDamage(Message) _hitactor self (Variables|Default|GetDamage) _hitbonename))
    (if _isvalidhit
      (if _isdead
        (Default|ComponentAddXP (Variables|Default|GetBP_XP_Component) _xp)
        (return)))
    (else
      (if (and (Utilities|DoesObjectImplementInterface _hitactor "/Script/UE_RIFLE.DamageInterface") (or (Variables|Default|GetIsModeFFA) (Variables|Default|GetIsModeTDM)))
        (Development|PrintString "Svr Process Hit : True" true true "(R=1.000000,G=0.000000,B=0.386642,A=1.000000)" 5.0)
        (Class|BPIDamagePlayer|PlayerTakeDamage(Message) _hitactor self HitResult (Variables|Default|GetDamage) true (Variables|Default|GetTeam%20ID))
        (else
          (Development|PrintString "Svr Process Hit : False" true true "(R=1.000000,G=0.000000,B=0.531326,A=1.000000)" 5.0)))
      (return))))

(fn SvrBulletTrace)

(fn GettDamageDirection
  (params (Attacker :type Actor%20Object%20Reference))
  (LocalVariables|SetLcl_DamageYaw (Math|Rotator|NormalizeAxis (- (.yaw (Math|Rotator|MakeRotfromZ (- (Transformation|GetActorLocation) (Transformation|GetActorLocation Attacker)))) (- (.yaw (Transformation|GetActorRotation)) 9e+01))))
  (if (< (LocalVariables|GetLcl_DamageYaw) 0.0)
    (if (Math|Float|InRange(Float) (LocalVariables|GetLcl_DamageYaw) -135.0 -45.0 true false)
      (LocalVariables|SetLcl_DamageDirection "NewEnumerator2")
      (elif (>= (LocalVariables|GetLcl_DamageYaw) -45.0)
        (LocalVariables|SetLcl_DamageDirection "NewEnumerator0")
        (else
          (LocalVariables|SetLcl_DamageDirection "NewEnumerator1"))))
    (elif (Math|Float|InRange(Float) (LocalVariables|GetLcl_DamageYaw) 45.0 135.0 false)
      (LocalVariables|SetLcl_DamageDirection "NewEnumerator3")
      (elif (<= (LocalVariables|GetLcl_DamageYaw) 45.0)
        (LocalVariables|SetLcl_DamageDirection "NewEnumerator0")
        (else
          (LocalVariables|SetLcl_DamageDirection "NewEnumerator1")))))
  (return (LocalVariables|GetLcl_DamageDirection)))

(fn GetHitMontage
  (params (DamageDirection :type E_DamageDirection%20Enum :default "NewEnumerator0"))
  (switch Utilities|FlowControl|Switch|SwitchonE_DamageDirection DamageDirection
    (:NewEnumerator0
      (LocalVariables|SetLcl_HitMontage 0))
    (:NewEnumerator1
      (LocalVariables|SetLcl_HitMontage 0))
    (:NewEnumerator2
      (LocalVariables|SetLcl_HitMontage 0))
    (:NewEnumerator3
      (LocalVariables|SetLcl_HitMontage 0)))
  (return (LocalVariables|GetLcl_HitMontage)))

(fn GetDeathMontage
  (params (DamageDirection :type E_DamageDirection%20Enum :default "NewEnumerator0"))
  (switch Utilities|FlowControl|Switch|SwitchonE_DamageDirection DamageDirection
    (:NewEnumerator0
      (LocalVariables|SetLcl_HitMontage "/Game/Character/Animations/Common/Char_Dead.Char_Dead"))
    (:NewEnumerator1
      (LocalVariables|SetLcl_HitMontage "/Game/Character/Animations/Common/Char_Dead.Char_Dead"))
    (:NewEnumerator2
      (LocalVariables|SetLcl_HitMontage "/Game/Character/Animations/Common/Char_Dead.Char_Dead"))
    (:NewEnumerator3
      (LocalVariables|SetLcl_HitMontage "/Game/Character/Animations/Common/Char_Dead.Char_Dead")))
  (return (LocalVariables|GetLcl_HitMontage)))

(fn TakeAIDamage
  (params (Attacker :type Actor%20Object%20Reference) (HitResult :type Hit%20Result%20Structure%20%28by%20ref%29) (DamageAmount :type Float%20%28double-precision%29))
  (bind (_bblockinghit _binitialoverlap _time _distance _location _impactpoint _normal _impactnormal) (Collision|BreakHitResult HitResult))
  (if (Variables|Default|GetIsAlive)
    (bind _output_get (Variables|Default|SetBP_Health (Math|Float|Clamp(Float) (- (Variables|Default|GetBP_Health) DamageAmount) 0.0 1e+03)))
    (CallFunction|ClientUpdateHUDHealth _output_get false)
    (bind _damagedirection (CallFunction|GettDamageDirection Attacker))
    (if (== (Variables|Default|GetBP_Health) 0.0)
      (Variables|Default|SetIsAlive false)
      (bind _hitmontage (CallFunction|GetDeathMontage _damagedirection))
      (CallFunction|MCAIMeleeImpact _impactpoint _impactnormal _hitmontage)
      (CallFunction|Die 0.0)
      (bind _asbp_shooter_game_mode (Utilities|Casting|CastToBP_ShooterGameMode (Game|GetGameMode)))
      (Default|GMEWPlayerDied _asbp_shooter_game_mode)
      (else
        (bind _hitmontage_2 (CallFunction|GetHitMontage _damagedirection))
        (CallFunction|MCAIMeleeImpact _impactpoint _impactnormal _hitmontage_2)))))

(fn TakePvPDamage
  (params (Attacker :type Actor%20Object%20Reference) (HitResult :type Hit%20Result%20Structure%20%28by%20ref%29) (DamageAmount :type Float%20%28double-precision%29) (AttackerTeamID :type Integer))
  (bind (_bblockinghit _binitialoverlap _time _distance _location _impactpoint _normal _impactnormal) (Collision|BreakHitResult HitResult))
  (if (Variables|Default|GetIsAlive)
    (Development|PrintString "Alive" (Variables|Default|GetIsAlive) true "(R=0.000000,G=0.035872,B=1.000000,A=1.000000)" 5.0)
    (if (or (and (Variables|Default|GetIsModeTDM) (!= AttackerTeamID (Variables|Default|GetTeam%20ID))) (Variables|Default|GetIsModeFFA))
      (bind _output_get (Variables|Default|SetHealth (Math|Float|Clamp(Float) (- (Variables|Default|GetHealth) DamageAmount) 0.0 1e+03)))
      (CallFunction|ClientUpdateHUDHealth _output_get false)
      (CallFunction|HUDCreateDaamageIndicator (Transformation|GetActorLocation Attacker))
      (bind _damagedirection (CallFunction|GettDamageDirection Attacker))
      (if (<= (Variables|Default|GetHealth) 0.0)
        (Variables|Default|SetIsAlive false)
        (bind _hitmontage (CallFunction|GetDeathMontage _damagedirection))
        (CallFunction|MCAIMeleeImpact _impactpoint _impactnormal _hitmontage)
        (CallFunction|Die (Variables|Default|GetRespawnDelay))
        (Variables|Default|GetBP_ShooterGameMode
          (:then
            _)
          (:else
            (bind _asbp_shooter_game_mode (Utilities|Casting|CastToBP_ShooterGameMode (Game|GetGameMode)))
            (Variables|Default|SetBP_ShooterGameMode _asbp_shooter_game_mode)))
        (bind _asbp_cplayer_base (Utilities|Casting|CastToBP_CPlayer_Base Attacker))
        (Default|GMPvPKilledPlayer (Variables|Default|GetBP_ShooterGameMode) (Variables|BP_CPlayer_Base_C|GetBP_SHooterPlayerController _asbp_cplayer_base) (Variables|Default|GetBP_SHooterPlayerController))
        (else
          (bind _hitmontage_2 (CallFunction|GetHitMontage _damagedirection))
          (CallFunction|MCAIMeleeImpact _impactpoint _impactnormal _hitmontage_2))))))