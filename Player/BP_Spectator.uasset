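; Spectator pawn that lets a player cycle through players with Q and E and respawn with F when allowed.
; On possession it shows spectator controls, and server events rebuild the player list, limited to teammates in Team Death Match.
; Cycling wraps the index, retries after short delays until it finds a living player, then targets attachment and updates the HUD name.
; The pawn destroys itself when unpossessed.
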(event Custom|Svr_UpdatePlayers
  (bind _attachedplayer (Variables|Default|GetAttachedPlayer))
  (bind _attachedplayer_2 (Variables|Default|GetAttachedPlayer))
  (switch Utilities|FlowControl|Switch|SwitchonE_GameModes (Variables|Default|GetCurrentGame%20Mode)
    (:NewEnumerator0
      (bind _outactors (Actor|GetAllActorsOfClass "/Game/Player/BP_CPlayer_Base.BP_CPlayer_Base_C" :!label _label))
      (Variables|Default|SetAllPlayers _outactors)
      (Utilities|IsValid _attachedplayer
        (:Is%20Valid
          (Variables|Default|SetCurrentPlayerIndex (Utilities|Array|FindItem (Variables|Default|GetAllPlayers) _attachedplayer)))))
    (:NewEnumerator1
      (goto _label))
    (:NewEnumerator2
      (Utilities|Array|Clear (Variables|Default|GetAllPlayers))
      (bind _outactors_2 (Actor|GetAllActorsOfClass "/Game/Player/BP_CPlayer_Base.BP_CPlayer_Base_C"))
      (for _array_element _outactors_2
        (if (== (Variables|/Game/Player/BP_CPlayer_Base.BP_CPlayer_Base_C|GetTeam%20ID _array_element) (Variables|Default|GetTeam%20ID))
          (Utilities|Array|Add (Variables|Default|GetAllPlayers) _array_element)))
      (Utilities|IsValid _attachedplayer_2
        (:Is%20Valid
          (Variables|Default|SetCurrentPlayerIndex (Utilities|Array|FindItem (Variables|Default|GetAllPlayers) _attachedplayer_2)))))))

(event Custom|Svr_AttachToPlayer
  (params (IncreaseIndex :type Boolean))
  (if IncreaseIndex
    (bind _result (Math|Integer|IncrementInt (Variables|Default|GetCurrentPlayerIndex) :!label _label)
      (:%20%20
        (if (>= _result (Utilities|Array|Length (Variables|Default|GetAllPlayers)))
          (Variables|Default|SetCurrentPlayerIndex 0))
        (if (Variables|/Game/Player/BP_CPlayer_Base.BP_CPlayer_Base_C|GetIsAlive (Utilities|Array|Get(acopy) (Variables|Default|GetAllPlayers) (Variables|Default|GetCurrentPlayerIndex)))
          (Variables|Default|SetAttachedPlayer 0)
          (elif (> (Utilities|Array|Length (Variables|Default|GetAllPlayers)) 1)
            (Utilities|FlowControl|Delay 0.1)
            (goto _label)
            (else
              (Utilities|FlowControl|Delay 0.5)
              (CallFunction|UpdatePlayers)
              (goto _label))))))
    (else
      (bind _result_2 (Math|Integer|DecrementInt (Variables|Default|GetCurrentPlayerIndex) :!label _label_2)
        (:%20%20
          (if (< _result_2 0)
            (Variables|Default|SetCurrentPlayerIndex (- (Utilities|Array|Length (Variables|Default|GetAllPlayers)) 1)))
          (if (Variables|/Game/Player/BP_CPlayer_Base.BP_CPlayer_Base_C|GetIsAlive (Utilities|Array|Get(acopy) (Variables|Default|GetAllPlayers) (Variables|Default|GetCurrentPlayerIndex)))
            (Variables|Default|SetAttachedPlayer 0)
            (elif (> (Utilities|Array|Length (Variables|Default|GetAllPlayers)) 1)
              (Utilities|FlowControl|Delay 0.1)
              (goto _label_2)
              (else
                (Utilities|FlowControl|Delay 0.5)
                (CallFunction|UpdatePlayers)
                (goto _label_2))))))))
  (Transformation|AttachActorToActor (Variables|Default|GetAttachedPlayer) "None" "SnapToTarget" "SnapToTarget" "KeepRelative" true)
  (Default|UpdateHUDSpectatorPlayerName (Variables|Default|GetBP_SHooterPlayerController) (.PlayerName (Utilities|Struct|BreakS_PlayerProfile (Variables|/Game/Framework/BP_ShooterPlayerController.BP_ShooterPlayerController_C|GetS_PlayerProfile (Variables|/Game/Player/BP_CPlayer_Base.BP_CPlayer_Base_C|GetBP_SHooterPlayerController (Variables|Default|GetAttachedPlayer)))))))

(event Custom|UpdatePlayers
  (bind _attachedplayer (Variables|Default|GetAttachedPlayer))
  (bind _attachedplayer_2 (Variables|Default|GetAttachedPlayer))
  (switch Utilities|FlowControl|Switch|SwitchonE_GameModes (Variables|Default|GetCurrentGame%20Mode)
    (:NewEnumerator0
      (bind _outactors (Actor|GetAllActorsOfClass "/Game/Player/BP_CPlayer_Base.BP_CPlayer_Base_C" :!label _label))
      (Variables|Default|SetAllPlayers _outactors)
      (Utilities|IsValid _attachedplayer
        (:Is%20Valid
          (Variables|Default|SetCurrentPlayerIndex (Utilities|Array|FindItem (Variables|Default|GetAllPlayers) _attachedplayer)))))
    (:NewEnumerator1
      (goto _label))
    (:NewEnumerator2
      (Utilities|Array|Clear (Variables|Default|GetAllPlayers))
      (bind _outactors_2 (Actor|GetAllActorsOfClass "/Game/Player/BP_CPlayer_Base.BP_CPlayer_Base_C"))
      (for _array_element _outactors_2
        (if (== (Variables|/Game/Player/BP_CPlayer_Base.BP_CPlayer_Base_C|GetTeam%20ID _array_element) (Variables|Default|GetTeam%20ID))
          (Utilities|Array|Add (Variables|Default|GetAllPlayers) _array_element)))
      (Utilities|IsValid _attachedplayer_2
        (:Is%20Valid
          (Variables|Default|SetCurrentPlayerIndex (Utilities|Array|FindItem (Variables|Default|GetAllPlayers) _attachedplayer_2)))))))

(event EventUnpossessed
  (params (OldController :type Controller%20Object%20Reference))
  (Actor|DestroyActor))

(event EventPossessed
  (params (NewController :type Controller%20Object%20Reference))
  (bind _asbp_shooter_player_controller (Utilities|Casting|CastToBP_ShooterPlayerController NewController))
  (bind _output_get (Variables|Default|SetBP_SHooterPlayerController _asbp_shooter_player_controller))
  (Default|ShowSpectatorControls _output_get)
  (CallFunction|UpdatePlayers)
  (CallFunction|SvrAttachtoPlayer true)
  (if (Networking|IsServer)
    (bind _asbp_shooter_game_mode (Utilities|Casting|CastToBP_ShooterGameMode (Game|GetGameMode)))
    (Variables|Default|SetCurrentGame%20Mode (Variables|/Game/Framework/BP_ShooterGameMode.BP_ShooterGameMode_C|GetGameMode _asbp_shooter_game_mode))
    (Variables|Default|SetTeam%20ID (Variables|/Game/Framework/BP_ShooterPlayerController.BP_ShooterPlayerController_C|GetTeamID (Variables|Default|GetBP_SHooterPlayerController)))))

(event Input|ActionEvents|InputActionPauseGame
  (params (Key :type Key%20Structure))
  (:Pressed
    (bind _asbp_shooter_game_instance (Utilities|Casting|CastToBP_ShooterGameInstance (Game|GetGameInstance)))
    (Default|TogglePauseGame _asbp_shooter_game_instance)))

(event Input|KeyboardEvents|F
  (params (Key :type Key%20Structure))
  (bind _bp_shooterplayercontroller (Variables|Default|GetBP_SHooterPlayerController))
  (:Pressed
    (if (Variables|/Game/Framework/BP_ShooterPlayerController.BP_ShooterPlayerController_C|GetIsRespawnEnabled _bp_shooterplayercontroller)
      (Variables|/Game/Framework/BP_ShooterPlayerController.BP_ShooterPlayerController_C|SetIsSpectating _bp_shooterplayercontroller false)
      (Variables|/Game/Framework/BP_ShooterPlayerController.BP_ShooterPlayerController_C|SetBP_Spectator _bp_shooterplayercontroller 0)
      (Default|RespawnAfterDeath _bp_shooterplayercontroller))))

(event Input|KeyboardEvents|Q
  (params (Key :type Key%20Structure))
  (:Pressed
    (CallFunction|SvrUpdatePlayers)
    (CallFunction|SvrAttachtoPlayer false)))

(event Input|KeyboardEvents|E
  (params (Key :type Key%20Structure))
  (:Pressed
    (CallFunction|SvrUpdatePlayers)
    (CallFunction|SvrAttachtoPlayer true)))

(fn ConstructionScript)