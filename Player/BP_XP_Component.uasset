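; Player component that tracks XP and level for BP_CPlayer_Base, with leveling capped at 10.
; Init loads the XP threshold map and reads saved values from player controller 0's profile struct.
; Adding XP runs on the server or locally controlled player, checks thresholds (allowing multi-level jumps), then writes back to the profile.
; The local controller also refreshes the HUD, saves XP and level, and plays a level-up animation.
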(event Custom|XP_Component_Init
  (CallFunction|SetupXPMap)
  (bind _asbp_cplayer_base (Utilities|Casting|CastToBP_CPlayer_Base (Components|GetOwner)))
  (Variables|Default|SetAs%20BP%20CPlayer%20Base _asbp_cplayer_base)
  (bind _asbp_shooter_player_controller (Utilities|Casting|CastToBP_ShooterPlayerController (Game|GetPlayerController 0)))
  (bind _output_get (Variables|Default|SetAs%20BP%20SHooter%20Player%20Controller _asbp_shooter_player_controller))
  (Variables|Default|SetPlayer%20XP (.Player_XP (Utilities|Struct|BreakS_PlayerProfile (Variables|/Game/Framework/BP_ShooterPlayerController.BP_ShooterPlayerController_C|GetS_PlayerProfile _output_get))))
  (Variables|Default|SetPlayer%20Level (.Player_Level (Utilities|Struct|BreakS_PlayerProfile (Variables|/Game/Framework/BP_ShooterPlayerController.BP_ShooterPlayerController_C|GetS_PlayerProfile _output_get))))
  (if (Pawn|IsLocalPlayerController (Variables|Default|GetAs%20BP%20SHooter%20Player%20Controller))
    (Default|UpdXPAmount (Variables|/Game/Framework/BP_ShooterPlayerController.BP_ShooterPlayerController_C|GetWB_IngameHUD (Variables|Default|GetAs%20BP%20SHooter%20Player%20Controller)))
    (Default|UpdXPLevel (Variables|/Game/Framework/BP_ShooterPlayerController.BP_ShooterPlayerController_C|GetWB_IngameHUD (Variables|Default|GetAs%20BP%20SHooter%20Player%20Controller)))))

(event Custom|ComponentAdd_XP
  (params (XpAmount :type Integer))
  (bind _as_bp_shooter_player_controller (Variables|Default|GetAs%20BP%20SHooter%20Player%20Controller))
  (bind _wb_ingamehud (Variables|/Game/Framework/BP_ShooterPlayerController.BP_ShooterPlayerController_C|GetWB_IngameHUD _as_bp_shooter_player_controller))
  (if (or (Networking|IsServer) (Pawn|IsLocallyControlled (Variables|Default|GetAs%20BP%20CPlayer%20Base)))
    (bind _output_get (Variables|Default|SetPlayer%20XP (+ (Variables|Default|GetPlayer%20XP) XpAmount)))
    (bind (_canlevelup _newlevel) (CallFunction|CheckforLevelUp _output_get))
    (if _canlevelup
      (Variables|Default|SetPlayer%20Level _newlevel))
    (CallFunction|UpdPlayerControllerProfile)
    (if (Pawn|IsLocalPlayerController _as_bp_shooter_player_controller)
      (Default|UpdXPAmount _wb_ingamehud)
      (Default|UpdXPLevel _wb_ingamehud)
      (Default|SaveXPandLevel _as_bp_shooter_player_controller)
      (if _canlevelup
        (Default|PlayUIanimLevelUp _wb_ingamehud)))))

(fn SetupXPMap
  (Variables|Default|SetXP_Map_Levels (.xp_map_levels (LocalVariables|GetS_XPandLevel)))
  (return))

(fn CheckforLevelUp
  (params (XPAmount :type Integer))
  (LocalVariables|SetLcl_CurrentPlrXP XPAmount)
  (LocalVariables|SetLcl_CurrentPlrLevel (Variables|Default|GetPlayer%20Level))
  (if (and (> (LocalVariables|GetLcl_CurrentPlrXP) (Utilities|Array|Get(acopy) (Variables|Default|GetXP_Map_Levels) (LocalVariables|GetLcl_CurrentPlrLevel))) (< (LocalVariables|GetLcl_CurrentPlrLevel) 10))
    (LocalVariables|SetLcl_CanLevelUp true)
    (bind _index (Utilities|FlowControl|ForLoopwithBreak (LocalVariables|GetLcl_CurrentPlrLevel) 10 :!label _label)
      (:LoopBody
        (if (not (> (LocalVariables|GetLcl_CurrentPlrXP) (Utilities|Array|Get(acopy) (Variables|Default|GetXP_Map_Levels) _index)))
          (LocalVariables|SetLcl_CurrentPlrLevel _index)
          (goto _label Break)))
      (:Completed
        (return (LocalVariables|GetLcl_CanLevelUp) (LocalVariables|GetLcl_CurrentPlrLevel))))
    (else
      (LocalVariables|SetLcl_CanLevelUp false)
      (return (LocalVariables|GetLcl_CanLevelUp) (LocalVariables|GetLcl_CurrentPlrLevel)))))

(fn UpdPlayerControllerProfile
  (Utilities|Struct|SetmembersinS_PlayerProfile (Variables|/Game/Framework/BP_ShooterPlayerController.BP_ShooterPlayerController_C|GetS_PlayerProfile (Variables|Default|GetAs%20BP%20SHooter%20Player%20Controller)) (Variables|Default|GetPlayer%20XP) (Variables|Default|GetPlayer%20Level))
  (return))